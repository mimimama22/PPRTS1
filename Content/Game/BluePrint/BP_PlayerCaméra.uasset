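; RTS camera pawn that moves, yaws and zooms via Enhanced Input, creates the HUD and drives unit selection and building placement.
; BuildMode enables Tick, which spawns one preview building through a DoOnce and snaps it to the cursor trace.
; Interact places it if allowed, deducting cost from player state resources, or otherwise selects the actor under the cursor.
; Action sends the selected actor a target or location message through cursor traces.
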(event Custom|BuildMode
  (params (RefSpawnBuild :type BP%20Build%20Base%20Class%20Reference))
  (Variables|Reference|SetRefSpawnBuild RefSpawnBuild)
  (bind _output_get (Variables|Parameter|SetIsBluidMode (not (Variables|Parameter|GetIsBluidMode))))
  (if _output_get
    (Actor|Tick|SetActorTickEnabled true)
    (else
      (Actor|Tick|SetActorTickEnabled false)
      (bind _currentbuild (Variables|Reference|GetCurrentBuild)
        (:then
          (Actor|DestroyActor _currentbuild))
        (:else)))))

(event Custom|ResetBuild
  (Utilities|FlowControl|DoOnce false) ; enters at Reset
)

(event Input|EnhancedActionEvents|EnhancedInputActionIA_Move
  (params (ActionValue :type Vector%202D%20Structure) (ElapsedSeconds :type Float%20%28double-precision%29) (TriggeredSeconds :type Float%20%28double-precision%29) (InputAction :type Input%20Action%20Object%20Reference :default "/Game/Game/input/Action/IA_Move.IA_Move"))
  (Pawn|Input|AddMovementInput (Math|Vector|GetRightVector (Variables|Default|Getcollision)) (.x ActionValue) false)
  (Pawn|Input|AddMovementInput (Math|Vector|GetForwardVector (Variables|Default|Getcollision)) (.y ActionValue) false))

(event Input|EnhancedActionEvents|EnhancedInputActionIA_Look
  (params (ActionValue :type Float%20%28double-precision%29) (ElapsedSeconds :type Float%20%28double-precision%29) (TriggeredSeconds :type Float%20%28double-precision%29) (InputAction :type Input%20Action%20Object%20Reference :default "/Game/Game/input/Action/IA_Look.IA_Look"))
  (bind _collision (Variables|Default|Getcollision))
  (bind _relativerotation (Variables|/Script/Engine.SceneComponent|GetRelativeRotation _collision))
  (Transformation|SetRelativeRotation (Variables|Default|Getcollision) (Math|Rotator|MakeRotator (.roll _relativerotation) (.pitch _relativerotation) (+ (.yaw _relativerotation) ActionValue)) false false))

(event Input|EnhancedActionEvents|EnhancedInputActionAI_UpCamera
  (params (ActionValue :type Float%20%28double-precision%29) (ElapsedSeconds :type Float%20%28double-precision%29) (TriggeredSeconds :type Float%20%28double-precision%29) (InputAction :type Input%20Action%20Object%20Reference :default "/Game/Game/input/Action/AI_UpCamera.AI_UpCamera"))
  (bind _springarm (Variables|Default|GetSpringArm))
  (Variables|/Script/Engine.SpringArmComponent|SetTargetArmLength _springarm (+ (* ActionValue -1e+02) (Variables|/Script/Engine.SpringArmComponent|GetTargetArmLength _springarm))))

(event Input|EnhancedActionEvents|EnhancedInputActionAI_Interaction
  (params (ActionValue :type Boolean) (ElapsedSeconds :type Float%20%28double-precision%29) (TriggeredSeconds :type Float%20%28double-precision%29) (InputAction :type Input%20Action%20Object%20Reference :default "/Game/Game/input/Action/AI_Interaction.AI_Interaction"))
  (bind _playerstate (Variables|GetPlayerState))
  (bind _asbp_custom_player_state (Utilities|Casting|CastToBP_CustomPlayerState _playerstate))
  (:Started
    (if (Variables|Parameter|GetIsBluidMode)
      (bind _currentbuild (Variables|Reference|GetCurrentBuild)
        (:then
          (if (Variables|/Game/Game/BluePrint/Building/BP_BuildBase.BP_BuildBase_C|GetCanBuild _currentbuild)
            (Default|Place (Variables|Reference|GetCurrentBuild))
            (Variables|/Game/Game/BluePrint/Building/BP_BuildBase.BP_BuildBase_C|SetIsBuild (Variables|Reference|GetCurrentBuild) false)
            (Class|BPIInteraction|NewTarget(Message) (Variables|Reference|GetRef%20Actor%20Interact) (Variables|Reference|GetCurrentBuild))
            (Variables|/Game/Game/BluePrint/Building/BP_BuildBase.BP_BuildBase_C|SetRef%20Player (Variables|Reference|GetCurrentBuild) self)
            (Variables|/Game/Game/BluePrint/BP_CustomPlayerState.BP_CustomPlayerState_C|SetRessources _asbp_custom_player_state (- (Variables|/Game/Game/BluePrint/BP_CustomPlayerState.BP_CustomPlayerState_C|GetRessources _asbp_custom_player_state) (Variables|/Game/Game/BluePrint/Building/BP_BuildBase.BP_BuildBase_C|GetCostBuild (Variables|Reference|GetCurrentBuild))))
            (Variables|Reference|SetCurrentBuild 0)
            (CallFunction|BuildMode)
            (CallFunction|ResetBuild)))
        (:else))
      (else
        (CallFunction|Interaction)))))

(event Input|EnhancedActionEvents|EnhancedInputActionAI_Action
  (params (ActionValue :type Boolean) (ElapsedSeconds :type Float%20%28double-precision%29) (TriggeredSeconds :type Float%20%28double-precision%29) (InputAction :type Input%20Action%20Object%20Reference :default "/Game/Game/input/Action/AI_Action.AI_Action"))
  (bind _array (Utilities|Array|MakeArray "ObjectTypeQuery2" "ObjectTypeQuery1" "ObjectTypeQuery3"))
  (bind _playercontrollerref (Variables|Reference|GetPlayerControllerRef))
  (bind (_hitresult _returnvalue) (Class|PlayerController|GetHitResultUnderCursorforObjects _playercontrollerref _array true))
  (bind (_bblockinghit _binitialoverlap _time _distance _location _impactpoint _normal _impactnormal _physmat _hitactor) (Collision|BreakHitResult _hitresult))
  (:Started
    (Variables|Reference|GetRef%20Actor%20Interact
      (:then
        (if _returnvalue
          (if (Utilities|DoesObjectImplementInterface _hitactor "/Game/Game/BluePrint/BPI_Interaction.BPI_Interaction_C")
            (Class|BPIInteraction|NewTarget(Message) (Variables|Reference|GetRef%20Actor%20Interact) _hitactor)
            (else
              (Class|BPIInteraction|NewLocation(Message) (Variables|Reference|GetRef%20Actor%20Interact) _location)))))
      (:else))))

(event EventBeginPlay
  (bind _returnvalue (Game|GetPlayerController 0))
  (bind _asplayer_controller (Utilities|Casting|CastToPlayerController (Pawn|GetController)))
  (Utilities|IsValid (PlayerController|LocalPlayerSubsystems|GetEnhancedInputLocalPlayerSubsystem _asplayer_controller)
    (:Is%20Valid
      (Input|AddMappingContext (PlayerController|LocalPlayerSubsystems|GetEnhancedInputLocalPlayerSubsystem _asplayer_controller) "/Game/Game/input/IMC_InputRTS.IMC_InputRTS" 0 "(bIgnoreAllPressedKeysUntilRelease=True,bForceImmediately=False,bNotifyUserSettings=False)")
      (Variables|Reference|SetPlayerControllerRef _returnvalue)
      (Variables|/Script/Engine.PlayerController|SetbShowMouseCursor _returnvalue true)
      (bind _returnvalue_2 (UserInterface|CreateWidget "/Game/Game/Widget/W_HUD.W_HUD_C"))
      (Variables|Reference|SetRefHUD _returnvalue_2)
      (Variables|/Game/Game/Widget/W_HUD.W_HUD_C|SetRefPlayer _returnvalue_2 self)
      (UserInterface|Viewport|AddtoViewport _returnvalue_2 0))))

(event EventTick
  (params (DeltaSeconds :type Float%20%28single-precision%29))
  (bind (_blockinghit _outhitlocation) (CallFunction|BuildTrace))
  (if (Variables|Parameter|GetIsBluidMode)
    (Utilities|FlowControl|Sequence
      (:then_0
        (Utilities|FlowControl|DoOnce false
          (:Completed
            (bind _returnvalue (Game|SpawnActorfromClass (Variables|Reference|GetRefSpawnBuild) (Transformation|GetActorTransform) "Undefined" "MultiplyWithRoot" 0 0))
            (bind _output_get (Variables|Reference|SetCurrentBuild _returnvalue))
            (Default|InitBuild _output_get)
            (Development|PrintString (Utilities|String|ToString(Boolean) (Variables|/Game/Game/BluePrint/Building/BP_BuildBase.BP_BuildBase_C|GetIsBuild _output_get)))
            (Transformation|SetActorRotation _output_get))))
      (:then_1
        (Variables|Reference|GetCurrentBuild
          (:then
            (if _blockinghit
              (Rendering|SetActorHiddenInGame (Variables|Reference|GetCurrentBuild) false)
              (Transformation|SetActorLocation (Variables|Reference|GetCurrentBuild) (+ _outhitlocation "") false false)
              (else
                (Rendering|SetActorHiddenInGame (Variables|Reference|GetCurrentBuild) true))))
          (:else))))))

(fn ConstructionScript)

(fn BuildTrace
  (bind _array (Utilities|Array|MakeArray "ObjectTypeQuery1"))
  (bind _playercontrollerref (Variables|Reference|GetPlayerControllerRef))
  (bind (_hitresult _returnvalue) (Class|PlayerController|GetHitResultUnderCursorforObjects _playercontrollerref _array true))
  (bind (_bblockinghit _binitialoverlap _time _distance _location _impactpoint _normal _impactnormal _physmat _hitactor _hitcomponent _hitbonename _bonename _hititem _elementindex _faceindex _tracestart _traceend) (Collision|BreakHitResult _hitresult))
  (if _returnvalue
    (return _bblockinghit _location)
    (else
      (return _bblockinghit _traceend))))

(fn Interaction
  (bind _array (Utilities|Array|MakeArray "ObjectTypeQuery2" "ObjectTypeQuery3"))
  (bind _playercontrollerref (Variables|Reference|GetPlayerControllerRef))
  (bind (_hitresult _returnvalue) (Class|PlayerController|GetHitResultUnderCursorforObjects _playercontrollerref _array true))
  (if _returnvalue
    (bind _ref_actor_interact (Variables|Reference|GetRef%20Actor%20Interact)
      (:then
        (Class|BPIInteraction|Deselect(Message) _ref_actor_interact (Variables|Reference|GetRefHUD)))
      (:else
        _))
    (bind _output_get (Variables|Reference|SetRef%20Actor%20Interact (.HitActor (Collision|BreakHitResult _hitresult))))
    (Class|BPIInteraction|Select(Message) _output_get (Variables|Reference|GetRefHUD) self)
    (else
      (bind _ref_actor_interact_2 (Variables|Reference|GetRef%20Actor%20Interact)
        (:then
          (Class|BPIInteraction|Deselect(Message) _ref_actor_interact_2 (Variables|Reference|GetRefHUD))
          (Variables|Reference|SetRef%20Actor%20Interact 0))
        (:else)))))