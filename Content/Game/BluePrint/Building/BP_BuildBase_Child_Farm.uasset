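; Farm building, a child of the build base Blueprint, that passively produces resources for its owning player.
; On BeginPlay it sets its health and fills the build mesh list with the farm meshes.
; StartFunctionPassive caches the custom player state from the player reference and starts a looping one-second timer, printing an error if the player is invalid.
; ProdRessources adds the resource increment to that player state's total.
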(event Custom|ProdRessources
  (bind _refplayer_state (Variables|Default|GetRefPlayer%20State))
  (Variables|/Game/Game/BluePrint/BP_CustomPlayerState.BP_CustomPlayerState_C|SetRessources _refplayer_state (+ (Variables|/Game/Game/BluePrint/BP_CustomPlayerState.BP_CustomPlayerState_C|GetRessources _refplayer_state) (Variables|Default|GetaddRessource))))

(event EventBeginPlay
  (bind _meshbuild (Variables|Default|GetMeshBuild))
  (|CallParentFunction)
  (Variables|Default|SetHeath 4e+01)
  (Utilities|Array|Clear _meshbuild)
  (Utilities|Array|Add _meshbuild "/Game/Toony_Tiny_RTS_Set_UE5/Meshes/Buildings/Construction/SM_Farm_0.SM_Farm_0")
  (Utilities|Array|Add _meshbuild "/Game/Toony_Tiny_RTS_Set_UE5/Meshes/Buildings/Construction/SM_Farm_1.SM_Farm_1")
  (Utilities|Array|Add _meshbuild "/Game/Toony_Tiny_RTS_Set_UE5/Meshes/Buildings/SM_Farm.SM_Farm"))

(event Collision|EventActorBeginOverlap
  (params (OtherActor :type Actor%20Object%20Reference))
  (|CallParentFunction OtherActor) ; This node is disabled and will not be called.\nDrag off pins to build functionality.
)

(event EventTick
  (params (DeltaSeconds :type Float%20%28single-precision%29))
  (|CallParentFunction DeltaSeconds) ; This node is disabled and will not be called.\nDrag off pins to build functionality.
)

(event EventStartFunctionPassive
  (bind _ref_player (Variables|Default|GetRef%20Player)
    (:then
      (bind _asbp_custom_player_state (Utilities|Casting|CastToBP_CustomPlayerState (Variables|/Script/Engine.Pawn|GetPlayerState _ref_player)))
      (Variables|Default|SetRefPlayer%20State _asbp_custom_player_state)
      (Utilities|Time|SetTimerbyEvent (EventDispatchers|CreateEvent :!event Custom|ProdRessources) 1.0 true))
    (:else
      (Development|PrintString "player NOt Valid" true true "(R=1.000000,G=0.000000,B=0.000000,A=1.000000)"))))

(fn ConstructionScript
  (|CallParentFunction))