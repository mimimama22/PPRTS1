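; Barracks building for a building system, a child Blueprint of the shared build base.
; On BeginPlay it runs the parent logic, then replaces the mesh list with three barracks meshes and sets its health and build cost.
; Selection registers the barracks with the HUD and switches the widget switcher to its panel, and deselection returns the switcher to the first panel.
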(event EventBeginPlay
  (bind _meshbuild (Variables|Default|GetMeshBuild))
  (|CallParentFunction)
  (Utilities|Array|Clear _meshbuild)
  (Utilities|Array|Add _meshbuild "/Game/Toony_Tiny_RTS_Set_UE5/Meshes/Buildings/Construction/SM_Barracks_0.SM_Barracks_0")
  (Utilities|Array|Add _meshbuild "/Game/Toony_Tiny_RTS_Set_UE5/Meshes/Buildings/Construction/SM_Barracks_1.SM_Barracks_1")
  (Utilities|Array|Add _meshbuild "/Game/Toony_Tiny_RTS_Set_UE5/Meshes/Buildings/SM_Barracks.SM_Barracks")
  (Variables|Default|SetHeath 5e+01)
  (Variables|Default|SetCostBuild 500))

(event EventSelect
  (params (RefHud :type W%20HUD%20Object%20Reference) (RefPlayer :type BP%20Player%20Caméra%20Object%20Reference))
  (Variables|/Game/Game/Widget/W_HUD.W_HUD_C|SetRefBuild RefHud self)
  (Variables|/Script/UMG.WidgetSwitcher|SetActiveWidgetIndex (Variables|/Game/Game/Widget/W_HUD.W_HUD_C|GetWidgetSwitcher_88 RefHud) 3))

(event EventDeselect
  (params (RefHUD :type W%20HUD%20Object%20Reference))
  (Variables|/Script/UMG.WidgetSwitcher|SetActiveWidgetIndex (Variables|/Game/Game/Widget/W_HUD.W_HUD_C|GetWidgetSwitcher_88 RefHUD) 0))

(fn ConstructionScript
  (|CallParentFunction))