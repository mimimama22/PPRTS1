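; QG building Blueprint, apparently a child of the shared build base, with little logic of its own.
; On BeginPlay it runs the parent logic, then sets its health variable (named Heath).
; Its construction script runs the parent's, then stores the static mesh's first material in MaterialStructure.
; The Select event only prints a debug string; overlap and Tick are disabled stubs.
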(event EventBeginPlay
  (|CallParentFunction)
  (Variables|Default|SetHeath 1e+02))

(event Collision|EventActorBeginOverlap
  (params (OtherActor :type Actor%20Object%20Reference))
  (|CallParentFunction OtherActor) ; This node is disabled and will not be called.\nDrag off pins to build functionality.
)

(event EventTick
  (params (DeltaSeconds :type Float%20%28single-precision%29))
  (|CallParentFunction DeltaSeconds) ; This node is disabled and will not be called.\nDrag off pins to build functionality.
)

(event EventSelect
  (Development|PrintString "select"))

(fn ConstructionScript
  (|CallParentFunction)
  (Variables|Default|SetMaterialStructure (Rendering|Material|GetMaterial (Variables|Default|GetStaticMesh) 0)))