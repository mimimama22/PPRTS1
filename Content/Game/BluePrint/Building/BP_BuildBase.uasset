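; BP_BuildBase is a building actor that handles placement preview, unit spawning and damage.
; InitBuild turns the mesh into an overlap-only preview, where begin and end overlap events toggle CanBuild and swap valid and invalid materials.
; Place applies the structure material and blocking collision but leaves IsBuild set.
; Select spawns a BP_AIBase at the Arrow transform, and AnyDamage drains Heath until the actor is destroyed.
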(event OnComponentBeginOverlap(StaticMesh)
  (params (OverlappedComponent :type Primitive%20Component%20Object%20Reference) (OtherActor :type Actor%20Object%20Reference) (OtherComp :type Primitive%20Component%20Object%20Reference) (OtherBodyIndex :type Integer) (bFromSweep :type Boolean) (SweepResult :type Hit%20Result%20Structure%20%28by%20ref%29))
  (if (Variables|Default|GetIsBuild)
    (Variables|Parameter|SetCanBuild false)
    (Rendering|Material|SetMaterial (Variables|Default|GetStaticMesh) 0 "/Game/Game/Material/Inst/M_BuildMat_NoValid_Inst.M_BuildMat_NoValid_Inst")
    (Development|PrintString "Hello")))

(event OnComponentEndOverlap(StaticMesh)
  (params (OverlappedComponent :type Primitive%20Component%20Object%20Reference) (OtherActor :type Actor%20Object%20Reference) (OtherComp :type Primitive%20Component%20Object%20Reference) (OtherBodyIndex :type Integer))
  (if (Variables|Default|GetIsBuild)
    (Variables|Parameter|SetCanBuild true)
    (Rendering|Material|SetMaterial (Variables|Default|GetStaticMesh) 0 "/Game/Game/Material/Inst/M_BuildMat_Inst_Valide.M_BuildMat_Inst_Valide")))

(event Custom|InitBuild
  (bind _staticmesh (Variables|Default|GetStaticMesh))
  (Rendering|Material|SetMaterial _staticmesh 0 "/Game/Game/Material/Inst/M_BuildMat_Inst_Valide.M_BuildMat_Inst_Valide")
  (Collision|SetCollisionResponsetoAllChannels _staticmesh "ECR_Overlap")
  (Variables|Default|SetIsBuild true))

(event Custom|Place
  (bind _staticmesh (Variables|Default|GetStaticMesh))
  (Rendering|Material|SetMaterial (Variables|Default|GetStaticMesh) 0 (Variables|Default|GetMaterialStructure))
  (Collision|SetCollisionEnabled _staticmesh "QueryAndPhysics")
  (Collision|SetCollisionResponsetoAllChannels _staticmesh "ECR_Block"))

(event EventBeginPlay
  (Development|PrintString (Utilities|String|ToString(Vector) (.BoxExtent (Collision|GetComponentBounds (Variables|Default|GetStaticMesh))))))

(event Collision|EventActorBeginOverlap
  (params (OtherActor :type Actor%20Object%20Reference)))

(event EventTick
  (params (DeltaSeconds :type Float%20%28single-precision%29)))

(event EventSelect
  (bind _returnvalue (Game|SpawnActorfromClass "/Game/Game/AI/BP_AIBase.BP_AIBase_C" (Transformation|GetWorldTransform (Variables|Default|GetArrow)) "AdjustIfPossibleButAlwaysSpawn" "MultiplyWithRoot" 0 0))
  (Development|PrintString (Utilities|GetDisplayName _returnvalue)))

(event Game|Damage|EventAnyDamage
  (params (Damage :type Float%20%28single-precision%29) (DamageType :type Damage%20Type%20Object%20Reference) (InstigatedBy :type Controller%20Object%20Reference) (DamageCauser :type Actor%20Object%20Reference))
  (Development|PrintString "damage")
  (bind _output_get (Variables|Default|SetHeath (- (Variables|Default|GetHeath) Damage)))
  (if (< _output_get 1.0)
    (Actor|DestroyActor)))

(fn ConstructionScript)