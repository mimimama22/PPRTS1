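; Starting headquarters (QG) building, a BP_BuildBase child that generates resources for the player and shows its own HUD panel when selected.
; BeginPlay sets health and town hall meshes, then after a short delay caches the player state and starts a looping timer, apparently driving ProdRessources to add AddRessource.
; Select and Deselect switch the HUD widget switcher.
; Timed mesh-stage swapping is left unconnected.
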(event Custom|ProdRessources
  (bind _refplayer_state (Variables|Default|GetRefPlayer%20State))
  (Variables|/Game/Game/BluePrint/BP_CustomPlayerState.BP_CustomPlayerState_C|SetRessources _refplayer_state (+ (Variables|/Game/Game/BluePrint/BP_CustomPlayerState.BP_CustomPlayerState_C|GetRessources _refplayer_state) (Variables|Default|GetaddRessource))))

(event EventBeginPlay
  (bind _meshbuild (Variables|Default|GetMeshBuild))
  (|CallParentFunction)
  (Variables|Default|SetHeath 1e+02)
  (Utilities|Array|Clear _meshbuild)
  (Utilities|Array|Add _meshbuild "/Game/Toony_Tiny_RTS_Set_UE5/Meshes/Buildings/Construction/SM_TownHall_0.SM_TownHall_0")
  (Utilities|Array|Add _meshbuild "/Game/Toony_Tiny_RTS_Set_UE5/Meshes/Buildings/Construction/SM_TownHall_1.SM_TownHall_1")
  (Utilities|Array|Add _meshbuild "/Game/Toony_Tiny_RTS_Set_UE5/Meshes/Buildings/SM_TownHall.SM_TownHall")
  (Utilities|FlowControl|Delay 0.2)
  (bind _asbp_player_caméra (Utilities|Casting|CastToBP_PlayerCaméra (Game|Player|GetPlayerPawn 0)))
  (Variables|Default|SetRef%20Player _asbp_player_caméra)
  (bind _ref_player (Variables|Default|GetRef%20Player)
    (:then
      (bind _asbp_custom_player_state (Utilities|Casting|CastToBP_CustomPlayerState (Variables|/Script/Engine.Pawn|GetPlayerState _ref_player)))
      (Variables|Default|SetRefPlayer%20State _asbp_custom_player_state)
      (Utilities|Time|SetTimerbyEvent (EventDispatchers|CreateEvent :!event Custom|ProdRessources) 3.0 true))
    (:else
      (Development|PrintString "player NOt Valid" true true "(R=1.000000,G=0.000000,B=0.000000,A=1.000000)"))))

(event EventDeselect
  (params (RefHUD :type W%20HUD%20Object%20Reference))
  (Variables|/Script/UMG.WidgetSwitcher|SetActiveWidgetIndex (Variables|/Game/Game/Widget/W_HUD.W_HUD_C|GetWidgetSwitcher_88 RefHUD) 0))

(event EventSelect
  (params (RefHud :type W%20HUD%20Object%20Reference) (RefPlayer :type BP%20Player%20Caméra%20Object%20Reference))
  (Variables|/Game/Game/Widget/W_HUD.W_HUD_C|SetRefBuild RefHud self)
  (Variables|/Script/UMG.WidgetSwitcher|SetActiveWidgetIndex (Variables|/Game/Game/Widget/W_HUD.W_HUD_C|GetWidgetSwitcher_88 RefHud) 2))

(fn ConstructionScript
  (|CallParentFunction)
  (Variables|Default|SetMaterialStructure (Rendering|Material|GetMaterial (Variables|Default|GetStaticMesh) 0)))