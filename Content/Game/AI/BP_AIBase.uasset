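; Base AI unit Blueprint that responds to select, deselect, move and target commands.
; When its AI master reference is valid, it forwards each command there, including its own location for move and target orders.
; Otherwise it acts alone, passing orders to its cached AI controller and toggling a mesh overlay material for selection.
; Any damage interrupts the mesh animation with a one-shot infantry hit reaction.
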(event EventBeginPlay
  (bind _asaic_aicharacter_base (Utilities|Casting|CastToAIC_AICharacterBase (AI|GetAIController self)))
  (Variables|Default|SetAs%20AIC%20AIBase _asaic_aicharacter_base))

(event EventDeselect
  (bind _refaimaster (Variables|Default|GetRefAIMaster)
    (:then
      (Default|DeselectUnit _refaimaster))
    (:else
      (Rendering|Material|SetOverlayMaterial (Variables|Character|GetMesh) 0 :!class /Script/Engine.MeshComponent))))

(event EventNewTarget
  (params (TargetActor :type Actor%20Object%20Reference))
  (bind _refaimaster (Variables|Default|GetRefAIMaster)
    (:then
      (Default|NewTagetUnit _refaimaster TargetActor (Transformation|GetActorLocation)))
    (:else
      (Default|SetNewTarget (Variables|Default|GetAs%20AIC%20AIBase) TargetActor))))

(event EventSelect
  (bind _refaimaster (Variables|Default|GetRefAIMaster)
    (:then
      (Default|Selectunit _refaimaster))
    (:else
      (Rendering|Material|SetOverlayMaterial (Variables|Character|GetMesh) "/Game/Game/Material/Inst/MI_OverlayBase.MI_OverlayBase" :!class /Script/Engine.MeshComponent))))

(event EventNewLocation
  (params (Position :type Vector :default "0, 0, 0"))
  (bind _refaimaster (Variables|Default|GetRefAIMaster)
    (:then
      (Default|NewlocationUnit _refaimaster Position (Transformation|GetActorLocation)))
    (:else
      (Default|SetNewPosition (Variables|Default|GetAs%20AIC%20AIBase) Position)
      (Development|PrintText "notvalid"))))

(event Game|Damage|EventAnyDamage
  (params (Damage :type Float%20%28single-precision%29) (DamageType :type Damage%20Type%20Object%20Reference) (InstigatedBy :type Controller%20Object%20Reference) (DamageCauser :type Actor%20Object%20Reference))
  (Audio|Components|Audio|Stop (Variables|Character|GetMesh))
  (Components|Animation|PlayAnimation (Variables|Character|GetMesh) "/Game/Toony_Tiny_RTS_Set_UE5/Animations/Units/Infantry/Anim_infantry_05_take_damage.Anim_infantry_05_take_damage" false))

(fn ConstructionScript)