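; BP_AIPlay is an early AI opponent prototype that places buildings around its headquarters and assigns a builder to them.
; BeginPlay caches the starting QG and a Batisseur builder, then starts a one-shot timer.
; SpawnBuild keeps a building spawned at a random point only if exactly one actor overlaps its box, otherwise destroys it.
; The builder-selection and repeating-spawn chain is disconnected, and Spawnenemy is empty.
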(event Custom|SpawnAroundQG
  (bind _refqg (Variables|Default|GetRefQG))
  (bind _staticmesh (Variables|/Game/Game/BluePrint/Building/BP_BuildBase.BP_BuildBase_C|GetStaticMesh _refqg))
  (bind (_origin _boxextent) (Collision|GetComponentBounds _staticmesh))
  (bind _returnvalue (Math|Random|RandomPointinBoundingBox _origin _boxextent))
  (Development|PrintString "Hello")
  (CallFunction|SpawnBuild (Variables|Default|GetClass) (Math|Transform|MakeTransform (+ (Math|Vector|MakeVector (.x _returnvalue) (.y _returnvalue) 0.0) (Transformation|GetActorLocation _refqg)) "0, 0, 0" "1.000000,1.000000,1.000000"))
  (Development|PrintString "Hello"))

(event Custom|Spawn%20enemy)

(event EventBeginPlay
  (Utilities|FlowControl|Delay 0.2)
  (bind _returnvalue (Actor|GetActorOfClass "/Game/Game/BluePrint/Building/BP_BuildBase_Child_QGStart.BP_BuildBase_Child_QGStart_C"))
  (Variables|Default|SetRefQG _returnvalue)
  (bind _returnvalue_2 (Actor|GetActorOfClass "/Game/Game/ALL_IA/AI/Batisseur/BP_AIBase_Child_Batisseur.BP_AIBase_Child_Batisseur_C"))
  (Development|PrintString (Utilities|GetDisplayName _returnvalue_2))
  (Utilities|Array|Add (Variables|Default|GetBuilderRef) _returnvalue_2)
  (Utilities|Time|SetTimerbyEvent (EventDispatchers|CreateEvent :!event Custom|SpawnAroundQG) 3.0))

(fn ConstructionScript)

(fn SpawnBuild
  (params (Class :type BP%20Build%20Base%20Class%20Reference) (SpawnTransform :type Transform))
  (bind _returnvalue (Game|SpawnActorfromClass Class SpawnTransform "Undefined" "MultiplyWithRoot" 0 0))
  (if (== (Utilities|Array|Length (Collision|GetOverlappingActors (Variables|/Game/Game/BluePrint/Building/BP_BuildBase.BP_BuildBase_C|GetBox _returnvalue) 0 :!class /Script/Engine.PrimitiveComponent)) 1)
    (Default|Place _returnvalue)
    (Default|NewTargetAI (Utilities|Array|Get(acopy) (Variables|Default|GetBuilderRef)) _returnvalue)
    (else
      (Actor|DestroyActor _returnvalue)
      (Development|PrintString "destroy"))))