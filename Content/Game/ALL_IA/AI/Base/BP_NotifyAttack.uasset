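; BP_NotifyAttack is an animation notify that deals melee weapon damage for AI characters.
; On notify, it sphere-traces between two right-hand weapon sockets for pawns and dynamic objects, ignoring the owner, with debug drawing enabled.
; A hit BP_AIBase takes fixed damage only if its Team differs from the owner's.
; Any other hit actor takes that damage without a team check.
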(fn ReceivedNotify
  (params (MeshComp :type Skeletal%20Mesh%20Component%20Object%20Reference) (Animation :type Anim%20Sequence%20Base%20Object%20Reference) (EventReference :type Anim%20Notify%20Event%20Reference%20Structure%20%28by%20ref%29))
  (bind _returnvalue (Components|GetOwner MeshComp))
  (bind (_outhit _returnvalue_2) (Collision|SphereTraceForObjects (Transformation|GetSocketLocation MeshComp "Weapon_Socket_R") (Transformation|GetSocketLocation MeshComp "Weapon_Socket_R_Sword") 1e+01 (Utilities|Array|MakeArray "ObjectTypeQuery3" "ObjectTypeQuery2") false (Utilities|Array|MakeArray _returnvalue) "ForDuration"))
  (if _returnvalue_2
    (bind _asbp_aibase (Utilities|Casting|CastToBP_AIBase (.HitActor (Collision|BreakHitResult _outhit)))
      (:then
        (if (!= (Variables|/Game/Game/ALL_IA/AI/Base/BP_AIBase.BP_AIBase_C|GetTeam _asbp_aibase) (Variables|/Game/Game/ALL_IA/AI/Base/BP_AIBase.BP_AIBase_C|GetTeam (.AsBP%20AIBase (Utilities|Casting|CastToBP_AIBase _returnvalue))))
          (Game|Damage|ApplyDamage (.HitActor (Collision|BreakHitResult _outhit)) 1e+01 0 _returnvalue :!label _label)
          (return false)))
      (:CastFailed
        (goto _label)))))