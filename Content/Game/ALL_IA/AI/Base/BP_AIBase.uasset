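; Base Blueprint for an AI unit that can be selected, ordered to a location or target, and damaged.
; Orders and selection route through RefAIMaster when valid, otherwise act directly on the AI controller or mesh overlay highlight, as the AI-suffixed events do.
; Damage retargets the attacker, reduces health, and plays a hit animation or destroys the actor at zero; the death montage is unconnected.
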(event Custom|SelectAI
  (Rendering|Material|SetOverlayMaterial (Variables|Character|GetMesh) "/Game/Game/Material/Inst/MI_OverlayBase.MI_OverlayBase" :!class /Script/Engine.MeshComponent))

(event Custom|DeselectAI
  (Rendering|Material|SetOverlayMaterial (Variables|Character|GetMesh) 0 :!class /Script/Engine.MeshComponent))

(event Custom|NewTargetAI
  (params (NewTarget :type Actor%20Object%20Reference))
  (Default|SetNewTarget (Variables|Default|GetAs%20AIC%20AIBase) NewTarget))

(event Custom|NewLocationAI
  (params (NewLocation :type Vector))
  (Default|SetNewPosition (Variables|Default|GetAs%20AIC%20AIBase) NewLocation))

(event EventBeginPlay
  (bind _asaic_aicharacter_base (Utilities|Casting|CastToAIC_AICharacterBase (AI|GetAIController self)))
  (Variables|Default|SetAs%20AIC%20AIBase _asaic_aicharacter_base))

(event EventNewTarget
  (params (TargetActor :type Actor%20Object%20Reference))
  (bind _refaimaster (Variables|Default|GetRefAIMaster)
    (:then
      (Default|NewTagetUnit _refaimaster TargetActor (Transformation|GetActorLocation)))
    (:else
      (Default|SetNewTarget (Variables|Default|GetAs%20AIC%20AIBase) TargetActor))))

(event EventSelect
  (params (RefHud :type W%20HUD%20Object%20Reference) (RefPlayer :type BP%20Player%20Caméra%20Object%20Reference))
  (bind _refaimaster (Variables|Default|GetRefAIMaster)
    (:then
      (Default|Selectunit _refaimaster))
    (:else
      (Rendering|Material|SetOverlayMaterial (Variables|Character|GetMesh) "/Game/Game/Material/Inst/MI_OverlayBase.MI_OverlayBase" :!class /Script/Engine.MeshComponent))))

(event EventNewLocation
  (params (Position :type Vector :default "0, 0, 0"))
  (bind _refaimaster (Variables|Default|GetRefAIMaster)
    (:then
      (Default|NewlocationUnit _refaimaster Position (Transformation|GetActorLocation)))
    (:else
      (Default|SetNewPosition (Variables|Default|GetAs%20AIC%20AIBase) Position)
      (Development|PrintText "notvalid"))))

(event Game|Damage|EventAnyDamage
  (params (Damage :type Float%20%28single-precision%29) (DamageType :type Damage%20Type%20Object%20Reference) (InstigatedBy :type Controller%20Object%20Reference) (DamageCauser :type Actor%20Object%20Reference))
  (Default|SetNewTarget (Variables|Default|GetAs%20AIC%20AIBase) DamageCauser)
  (bind _output_get (Variables|Default|Setheath (Math|Float|Truncate (- (Variables|Default|Getheath) Damage))))
  (Development|PrintString (Utilities|String|ToString(Integer) _output_get))
  (if (> _output_get 0)
    (Components|Animation|PlayAnimation (Variables|Character|GetMesh) "/Game/Toony_Tiny_RTS_Set_UE5/Animations/Units/Infantry/Anim_infantry_05_take_damage.Anim_infantry_05_take_damage" false)
    (else
      (Actor|DestroyActor))))

(event EventDeselect
  (params (RefHUD :type W%20HUD%20Object%20Reference))
  (bind _refaimaster (Variables|Default|GetRefAIMaster)
    (:then
      (Default|DeselectUnit _refaimaster))
    (:else
      (Rendering|Material|SetOverlayMaterial (Variables|Character|GetMesh) 0 :!class /Script/Engine.MeshComponent))))

(fn ConstructionScript)