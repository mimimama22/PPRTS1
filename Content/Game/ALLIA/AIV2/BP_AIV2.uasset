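; BP_AIV2 is a selectable AI unit that accepts move and target commands.
; Select and Deselect apply or clear an overlay material on all its skeletal mesh components to show selection.
; NewLocation and NewTarget pass a position or target actor straight to the AI controller reference, RefAIC.
; Possession only prints a debug greeting, and no other gameplay logic lives in these graphs.
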(event EventBeginPlay)

(event Collision|EventActorBeginOverlap
  (params (OtherActor :type Actor%20Object%20Reference)))

(event EventTick
  (params (DeltaSeconds :type Float%20%28single-precision%29)))

(event EventSelect
  (params (RefHud :type W%20HUD%20Object%20Reference) (RefPlayer :type BP%20Player%20Caméra%20Object%20Reference))
  (for _array_element (Actor|GetComponentsByClass "/Script/Engine.SkeletalMeshComponent")
    (Rendering|Material|SetOverlayMaterial _array_element "/Game/Game/Material/Inst/MI_OverlayBase.MI_OverlayBase" :!class /Script/Engine.MeshComponent)))

(event EventDeselect
  (params (RefHUD :type W%20HUD%20Object%20Reference))
  (for _array_element (Actor|GetComponentsByClass "/Script/Engine.SkeletalMeshComponent")
    (Rendering|Material|SetOverlayMaterial _array_element 0 :!class /Script/Engine.MeshComponent)))

(event EventNewLocation
  (params (Position :type Vector :default "0, 0, 0"))
  (Default|NewPosition (Variables|Default|GetRefAIC) Position))

(event EventNewTarget
  (params (TargetActor :type Actor%20Object%20Reference))
  (Default|NewTarget (Variables|Default|GetRefAIC) TargetActor))

(event EventPossessed
  (params (NewController :type Controller%20Object%20Reference))
  (Development|PrintString "Hello"))

(fn ConstructionScript)