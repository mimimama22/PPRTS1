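; Builder (Batisseur) AI unit, a child of an AI base Blueprint, that changes the HUD when selected.
; Select and Deselect call their parent versions, then flip a widget switcher on the passed HUD reference between the selected and default panels.
; GoBuild is an empty event, so no building logic exists in this graph.
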(event Custom|GoBuild)

(event EventBeginPlay
  (|CallParentFunction) ; This node is disabled and will not be called.\nDrag off pins to build functionality.
)

(event Collision|EventActorBeginOverlap
  (params (OtherActor :type Actor%20Object%20Reference)))

(event EventTick
  (params (DeltaSeconds :type Float%20%28single-precision%29)))

(event EventSelect
  (params (RefHud :type W%20HUD%20Object%20Reference) (RefPlayer :type BP%20Player%20Caméra%20Object%20Reference))
  (|CallParentFunction RefHud 0)
  (Class|WidgetSwitcher|SetActiveWidgetIndex (Variables|/Game/Game/Widget/W_HUD.W_HUD_C|GetWidgetSwitcher_88 RefHud) 1))

(event EventDeselect
  (params (RefHUD :type W%20HUD%20Object%20Reference))
  (|CallParentFunction RefHUD)
  (Variables|/Script/UMG.WidgetSwitcher|SetActiveWidgetIndex (Variables|/Game/Game/Widget/W_HUD.W_HUD_C|GetWidgetSwitcher_88 RefHUD) 0))

(fn ConstructionScript
  (|CallParentFunction))