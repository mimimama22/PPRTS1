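; BP_AIPlay is an actor that scripts a timed select and deselect of a builder AI when play begins.
; After a short delay, it finds a BP_AIBase_Child_Batisseur in the level and adds it to its BuilderRef array.
; It then calls SelectAI on that builder, waits ten seconds and calls DeselectAI, printing a debug string at each step.
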(event EventBeginPlay
  (Utilities|FlowControl|Delay 0.2)
  (bind _returnvalue (Actor|GetActorOfClass "/Game/Game/ALLIA/AI/Batisseur/BP_AIBase_Child_Batisseur.BP_AIBase_Child_Batisseur_C"))
  (Utilities|Array|Add (Variables|Default|GetBuilderRef) _returnvalue)
  (Utilities|FlowControl|Delay 1.0)
  (Default|SelectAI (Utilities|Array|Get(acopy) (Variables|Default|GetBuilderRef)))
  (Development|PrintString "select")
  (Utilities|FlowControl|Delay 1e+01)
  (Default|DeselectAI (Utilities|Array|Get(acopy) (Variables|Default|GetBuilderRef)))
  (Development|PrintString "deselect"))

(event Collision|EventActorBeginOverlap
  (params (OtherActor :type Actor%20Object%20Reference)))

(event EventTick
  (params (DeltaSeconds :type Float%20%28single-precision%29)))

(fn ConstructionScript)